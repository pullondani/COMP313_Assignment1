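; Player Blueprint for a rolling ball that moves, takes damage and can pause the game.
; Horizontal and Vertical axis inputs share one impulse on the Sphere, scaled by Speed.
; Overlapping an Arrow plays a world camera shake at the player's location.
; Damage lowers Health and refreshes the UI through MyGameMode, which also handles pausing and the loss at zero health.
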(event `InputAxis|Horizontal`
  (params (AxisValue :type "Float (single-precision)"))
  ;[1 1 1] Move a ball
  (`PrimitiveComponent.AddImpulse` (`self.Sphere`) (* (`KismetMathLibrary.MakeVector` AxisValue (stale `InputAxis|Vertical` AxisValue)) (`self.Speed`)) "None" false :!label _label))

(event `InputAxis|Vertical`
  (params (AxisValue :type "Float (single-precision)"))
  ;[1 1 1] Move a ball
  (goto _label))

(event `self.ReceiveActorBeginOverlap`
  (params (OtherActor :type "Actor Object Reference"))
  ;[1 1 1] Camera Shake On Hit
  (cast `/Game/Blueprints/Arrow` OtherActor)
  (`GameplayStatics.PlayWorldCameraShake` "/Game/Blueprints/BP_OnHitCameraShake.BP_OnHitCameraShake_C" (`self.K2_GetActorLocation`) 0.0 500.0))

(event `self.ReceiveAnyDamage`
  (params (Damage :type "Float (single-precision)") (DamageType :type "DamageType Object Reference") (InstigatedBy :type "Controller Object Reference") (DamageCauser :type "Actor Object Reference"))
  (bind _returnvalue (`GameplayStatics.GetGameMode`))
  ;[1 1 1] Set Player Health
  (bind _output_get (set `self.Health` (- (`self.Health`) (`KismetMathLibrary.FTrunc` Damage))))
  (bind _asmy_game_mode (cast `/Game/MyGameMode` _returnvalue))
  (`/Game/UI/UI_GameUI.Update Health` (`/Game/MyGameMode.currentUI` _asmy_game_mode))
  (if (<= _output_get 0)
    (bind _asmy_game_mode_2 (cast `/Game/MyGameMode` _returnvalue))
    (`/Game/MyGameMode.Lose Game` _asmy_game_mode_2)))

(event `InputAction|Pause`
  (params (Key :type "Key Structure"))
  ;[1 1 1] Press Pause
  (:`Pressed`
    (bind _asmy_game_mode (cast `/Game/MyGameMode` (`GameplayStatics.GetGameMode`)))
    (`/Game/MyGameMode.Pause Game` _asmy_game_mode)))

(fn `UserConstructionScript`)