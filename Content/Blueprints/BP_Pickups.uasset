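; BP_Pickups is a collectible pickup actor that spins in place and awards points when the player touches it.
; Tick applies a frame-rate independent local rotation built from roll, pitch and yaw speed variables.
; On overlap with BP_Player it destroys itself, then calls UpdatePoints on MyGameMode.
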(event `self.ReceiveTick`
  (params (DeltaSeconds :type "Float (single-precision)"))
  ;[1 1 1] Rotate cube
  (`self.K2_AddActorLocalRotation` (* (`KismetMathLibrary.MakeRotator` (`self.Roll Speed`) (`self.Pitch Speed`) (`self.Yaw Speed`)) DeltaSeconds)))

(event `self.ReceiveActorBeginOverlap`
  (params (OtherActor :type "Actor Object Reference"))
  ;[1 1 1] Collect Pickup
  (cast `/Game/Blueprints/BP_Player` OtherActor)
  (`self.K2_DestroyActor`)
  (bind _asmy_game_mode (cast `/Game/MyGameMode` (`GameplayStatics.GetGameMode`)))
  (`/Game/MyGameMode.Update Points` _asmy_game_mode))

(fn `UserConstructionScript`)